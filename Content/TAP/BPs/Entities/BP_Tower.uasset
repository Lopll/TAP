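; BP_Tower is an enemy tower entity with an HP readout that attacks by summoning units.
; HPCounter text is set from the health component on BeginPlay and updated on each health change.
; Attack ignores its target and spawns an AllyClass actor at a random reachable point nearby.
; It writes the TeamDark tag to make the spawn hostile to the player, then spawns that unit's AI controller to possess it.
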(event `self.ReceiveBeginPlay`
  (`parent.ReceiveBeginPlay`)
  (`TextRenderComponent.K2_SetText` (`self.HP_Counter`) (`KismetTextLibrary.Conv_IntToText` (`/Game/TAP/BPs/ActorComponents/BP_HealthComponent.HP` (`self.BP_HealthComponent`)))))

(event `self.OnHealthChanged`
  (params (HP :type Integer))
  (`TextRenderComponent.K2_SetText` (`self.HP_Counter`) (`KismetTextLibrary.Conv_IntToText` HP)))

(fn `Attack`
  (params (AttackTarget :type "/Game/TAP/BPs/Entities/BP_Entity Object Reference"))
  (`parent.Attack` null)
  ;[1 1 1] Spawn
  (bind _returnvalue (`|SpawnActorFromClass` (`self.AllyClass`) (`KismetMathLibrary.MakeTransform` (`NavigationSystemV1.K2_GetRandomReachablePointInRadius` (`self.K2_GetActorLocation`) 400.0 null null)) "Undefined" "OverrideRootScale" self null))
  (bind _output_get (set `self.LastCreatedAlly` _returnvalue))
  (`KismetArrayLibrary.Array_Set` (`Actor.Tags` _output_get) 0 "TeamDark") ; MakeSpeawnActorAnEnemyForThePlayer
  (bind _returnvalue_2 (`|SpawnActorFromClass` (`/Game/TAP/BPs/Entities/BP_Entity.AIController` (`self.LastCreatedAlly`)) (`KismetMathLibrary.MakeTransform` (0.0 0.0 0.0)) "Undefined" "OverrideRootScale" null null))
  (set `self.LastCreatedAllyController` _returnvalue_2)
  (`Controller.Possess` (`self.LastCreatedAllyController`) (`self.LastCreatedAlly`)))

(fn `UserConstructionScript`
  (`parent.UserConstructionScript`))