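; BP_Player is the player pawn, with health, mana, a camera and a world-space cursor marker.
; On begin play it activates the camera, caches the BP_PlayerController and seeds its HUD from the health and mana components, then forwards later changes.
; Each tick, a visibility trace under the mouse places CursorToWorld on the hit point, aligned to the surface normal.
; Death runs the parent logic, then reloads the current level.
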(event `self.ReceiveBeginPlay`
  ;[1 1 1] BeginPlay
  (`ActorComponent.Activate` (`self.Camera`) false)
  (bind _asbp_player_controller (cast `/Game/TAP/BPs/Controllers/BP_PlayerController` (`GameplayStatics.GetPlayerController` 0)))
  (bind _output_get (set `self.PlayerController` _asbp_player_controller))
  (bind _hud (`/Game/TAP/BPs/Controllers/BP_PlayerController.HUD` _output_get))
  (`/Game/TAP/GUI/WB_HUD.SetHP` _hud (`/Game/TAP/BPs/ActorComponents/BP_HealthComponent.HP` (`self.BP_HealthComponent`)))
  (`/Game/TAP/GUI/WB_HUD.SetMP` _hud (`/Game/TAP/BPs/ActorComponents/BP_ManaComponent.Mana` (`self.BP_ManaComponent`))))

(event `self.ReceiveTick`
  (params (DeltaSeconds :type "Float (single-precision)"))
  (bind (_bblockinghit _binitialoverlap _time _distance _location _impactpoint _normal _impactnormal) (`GameplayStatics.BreakHitResult` (`PlayerController.GetHitResultUnderCursorByChannel` (`GameplayStatics.GetPlayerController` 0) "TraceTypeQuery1" true)))
  ;[1 1 1] Tick
  (`SceneComponent.K2_SetWorldLocationAndRotation` (`self.CursorToWorld`) _location (`KismetMathLibrary.MakeRotationFromAxes` _impactnormal) false false))

(event `self.OnHealthChanged`
  (params (HP :type Integer))
  ;[1 1 1] Set stats
  (`/Game/TAP/GUI/WB_HUD.SetHP` (`/Game/TAP/BPs/Controllers/BP_PlayerController.HUD` (`self.PlayerController`)) HP))

(event `self.OnManaChanged`
  (params (MP :type Integer))
  ;[1 1 1] Set stats
  (`/Game/TAP/GUI/WB_HUD.SetMP` (`/Game/TAP/BPs/Controllers/BP_PlayerController.HUD` (`self.PlayerController`)) MP))

(fn `Death`
  (`parent.Death`)
  (bind _returnvalue (`GameplayStatics.GetCurrentLevelName` true))
  (`GameplayStatics.OpenLevel` (`KismetStringLibrary.Conv_StringToName` _returnvalue)))

(fn `UserConstructionScript`
  (`parent.UserConstructionScript`))