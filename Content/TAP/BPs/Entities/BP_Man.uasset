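; BP_Man is a combat unit entity that builds on a parent class and shows its health on an HP counter.
; After a short delay on BeginPlay, its first tag picks the mesh material: Mushrooms for Team Light, tree bark otherwise.
; Health changes from BPHealthComponent update the counter text.
; Attack triggers the target's damage reaction, subtracts IDamage from its HP and changes state, while Death destroys the actor.
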(event `self.ReceiveBeginPlay`
  (`parent.ReceiveBeginPlay`)
  (`TextRenderComponent.K2_SetText` (`self.HP_Counter`) (`KismetTextLibrary.Conv_IntToText` (`/Game/TAP/BPs/ActorComponents/BP_HealthComponent.HP` (`self.BP_HealthComponent`)))) ; SetHPCounter
  (`KismetSystemLibrary.Delay` 0.5)
  (switch `name` (`|GetArrayItem` (`self.Tags`))
    (:`Default`
      (`PrimitiveComponent.SetMaterial` (`self.Mesh`) 0 "/Game/TAP/Models/Nature/FBX/Bark_NormalTree.Bark_NormalTree" :!label _label))
    (:`TeamLight`
      (`PrimitiveComponent.SetMaterial` (`self.Mesh`) 0 "/Game/TAP/Models/Nature/FBX/Mushrooms.Mushrooms"))
    (:`TeamDark`
      (goto _label))))

(event `self.ReceiveTick`
  (params (DeltaSeconds :type "Float (single-precision)"))
  (`parent.ReceiveTick` DeltaSeconds))

(event `self.OnHealthChanged`
  (params (HP :type Integer))
  (`TextRenderComponent.K2_SetText` (`self.HP_Counter`) (`KismetTextLibrary.Conv_IntToText` HP)))

(fn `Attack`
  (params (AttackTarget :type "/Game/TAP/BPs/Entities/BP_Entity Object Reference"))
  (`parent.Attack` AttackTarget)
  (`self.OnDamageTaken` AttackTarget)
  (`/Game/TAP/BPs/ActorComponents/BP_HealthComponent.addHP` (`/Game/TAP/BPs/Entities/BP_Entity.BP_HealthComponent` AttackTarget) (* (`self.iDamage`) -1))
  (set `self.eCurrentState` "NewEnumerator2"))

(fn `Death`
  (`self.K2_DestroyActor`))

(fn `UserConstructionScript`
  (`parent.UserConstructionScript`))