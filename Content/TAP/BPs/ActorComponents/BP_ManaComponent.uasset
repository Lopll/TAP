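; BP_ManaComponent is an actor component that stores and regenerates mana for a BP_Entity owner, which it caches on BeginPlay.
; Tick passes ManaRecoverSpeed to AddMana every frame, without scaling by delta time.
; AddMana applies the delta under a ChangingMana guard, flooring at zero and setting a hardcoded 100 when the sum exceeds MaxMana.
; It then notifies the owner through OnManaChanged and returns the new value.
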(event `self.ReceiveBeginPlay`
  (bind _asbp_entity (cast `/Game/TAP/BPs/Entities/BP_Entity` (`self.GetOwner`)))
  (set `self.Owner` _asbp_entity))

(event `self.ReceiveTick`
  (params (DeltaSeconds :type "Float (single-precision)"))
  (`self.addMana` (`self.manaRecoverSpeed`)))

(fn `addMana`
  (params (delta :type Integer))
  (returns (Mana :type Integer))
  (bind _mana (`self.Mana`))
  (bind _returnvalue (+ delta (`self.Mana`)))
  (if (not (`self.changingMana`))
    (set `self.changingMana` true)
    (if (> _returnvalue (`self.MaxMana`))
      (set `self.Mana` 100)
      (elif (< _returnvalue 0)
        (set `self.Mana` 0)
        (else
          (set `self.Mana` _returnvalue))))
    (set `self.changingMana` false)
    (`/Game/TAP/BPs/Entities/BP_Entity.OnManaChanged` (`self.Owner`) _mana)
    (return _mana)))