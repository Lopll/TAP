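; Health component for a BP_Entity owner that tracks HP and handles regeneration and death.
; Tick adds HPRecoverSpeed every frame while recovery is enabled, without delta-time scaling.
; AddHP uses a ChangingHP guard, setting HP to a hardcoded 100 when the sum exceeds MaxHP.
; A sum at or below zero calls Death on the owner, leaving HP unchanged and the guard set.
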(event `self.ReceiveTick`
  (params (DeltaSeconds :type "Float (single-precision)"))
  (if (`self.ableToRecoverHP`)
    (`self.addHP` (`self.HPRecoverSpeed`))))

(fn `addHP`
  (params (delta :type Integer))
  (returns (Mana :type Integer))
  (bind _returnvalue (+ delta (`self.HP`)))
  (if (not (`self.changingHP`))
    (set `self.changingHP` true)
    (if (> _returnvalue (`self.MaxHP`))
      (set `self.HP` 100)
      (set `self.changingHP` false :!label _label)
      (return (`self.HP`))
      (elif (<= _returnvalue 0)
        (bind _asbp_entity (cast `/Game/TAP/BPs/Entities/BP_Entity` (`self.GetOwner`)))
        (`/Game/TAP/BPs/Entities/BP_Entity.Death` _asbp_entity)
        (else
          (set `self.HP` _returnvalue)
          (goto _label))))))