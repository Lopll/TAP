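; AI controller for the StoneMan that picks a target from sensed actors, intended for entities outside its team.
; A sensing event switches on the pawn's current state: Waiting tries to take the new target immediately.
; Attacking and Following switch only if the stimulus passes a distance check against the current Blackboard target, meant to favor the closer one.
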(event `CustomEvent`
  (params (Actor :type "Actor Object Reference") (Stimulus :type "AIStimulus Structure"))
  (bind _returnvalue (`self.K2_GetActorLocation` (`self.SelfPawn`)))
  ;[1 1 1] If not our team entity sensed, then set it as a target
  (switch `/Game/TAP/BPs/Enums/E_EntityStates` (`/Game/TAP/BPs/Entities/BP_Entity.eCurrentState` (`self.SelfPawn`))
    (:`NewEnumerator0`
      (if (< (`KismetMathLibrary.Vector_Distance` (`.StimulusLocation` (break `AIStimulus` Stimulus)) _returnvalue) (`KismetMathLibrary.Vector_Distance` _returnvalue (`self.K2_GetActorLocation` (cast `Actor` (`BlackboardComponent.GetValueAsObject` (`self.Blackboard`) (`self.TargetName`)) :!pure true)))) :!label _label
        (`self.TryToSetNewTarget` Actor :!label _label_2)))
    (:`NewEnumerator1`
      (goto _label))
    (:`NewEnumerator2`
      (goto _label_2))))

(fn `UserConstructionScript`
  (`parent.UserConstructionScript`))